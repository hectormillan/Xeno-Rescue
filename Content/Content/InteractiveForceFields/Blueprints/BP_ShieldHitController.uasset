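; Shield hit controller that plays an animated force-field impact effect for a struck static or skeletal mesh.
; OnImpact copies a static mesh onto itself or reinitializes the passed skeletal mesh, then picks from HitMaterials by matching index in MaterialsToInteract, with MaterialOverwrite able to bypass the match.
; It applies a dynamic instance across material slots, and a timeline per mesh type drives its HitPosition and Phase parameters.
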(event EventOnImpact
  (params (Location :type Vector :default "0, 0, 0") (Mesh :type Static%20Mesh%20Component%20Object%20Reference) (Material :type Material%20Interface%20Object%20Reference) (MaterialOverwrite :type Integer) (SkeletalMesh :type Skeletal%20Mesh%20Component%20Object%20Reference))
  (Utilities|IsValid SkeletalMesh
    (:Is%20Valid
      (Class|SkinnedMeshComponent|SetSkeletalMesh (Variables|Default|GetSkeletalMesh) (Variables|/Script/Engine.SkinnedMeshComponent|GetSkeletalMesh SkeletalMesh) true)
      (for (_array_element _array_index) (Variables|Default|GetMaterialsToInteract)
        (if (== MaterialOverwrite 0)
          (if (== Material _array_element)
            (bind _returnvalue (Rendering|Material|CreateDynamicMaterialInstance 0 (Utilities|Array|Get(acopy) (Variables|Default|GetHitMaterials) _array_index) "None" :!class /Script/Engine.PrimitiveComponent :!label _label))
            (bind _output_get (Variables|Default|SetDynamicMaterial _returnvalue))
            (for _index (range 0 (Utilities|Array|Length (Rendering|Material|GetMaterials SkeletalMesh)))
              (Rendering|Material|SetMaterial _index _output_get)
              (Rendering|Material|SetMaterial (Variables|Default|GetSkeletalMesh) _index _output_get))
            (bind _time (Timeline|Timeline_0 PlayFromStart)
              (:Update
                (Rendering|Material|SetVectorParameterValue (Variables|Default|GetDynamicMaterial) "HitPosition" (Math|Conversions|ToLinearColor(Vector) (+ (Transformation|GetWorldLocation SkeletalMesh) Location)) :!class /Script/Engine.MaterialInstanceDynamic)
                (Rendering|Material|SetScalarParameterValue (Variables|Default|GetDynamicMaterial) "Phase" _time :!class /Script/Engine.MaterialInstanceDynamic))))
          (elif (== MaterialOverwrite 2)
            (goto _label)
            (else
              (goto _label))))))
    (:Is%20Not%20Valid
      (Utilities|IsValid Mesh
        (:Is%20Valid
          (Components|StaticMesh|SetStaticMesh (Variables|/Script/Engine.StaticMeshComponent|GetStaticMesh Mesh))
          (for (_array_element_2 _array_index_2) (Variables|Default|GetMaterialsToInteract)
            (if (== MaterialOverwrite 0)
              (if (== Material _array_element_2)
                (bind _returnvalue_2 (Rendering|Material|CreateDynamicMaterialInstance 0 (Utilities|Array|Get(acopy) (Variables|Default|GetHitMaterials) _array_index_2) "None" :!class /Script/Engine.PrimitiveComponent :!label _label_2))
                (bind _output_get_2 (Variables|Default|SetDynamicMaterial _returnvalue_2))
                (for _index_2 (range 0 (Utilities|Array|Length (Rendering|Material|GetMaterials Mesh)))
                  (Rendering|Material|SetMaterial _index_2 _output_get_2)
                  (Rendering|Material|SetMaterial (Variables|Default|GetSkeletalMesh) _index_2 _output_get_2))
                (bind _time_2 (Timeline|Timeline PlayFromStart)
                  (:Update
                    (Rendering|Material|SetVectorParameterValue (Variables|Default|GetDynamicMaterial) "HitPosition" (Math|Conversions|ToLinearColor(Vector) (+ (Transformation|GetWorldLocation Mesh) Location)) :!class /Script/Engine.MaterialInstanceDynamic)
                    (Rendering|Material|SetScalarParameterValue (Variables|Default|GetDynamicMaterial) "Phase" _time_2 :!class /Script/Engine.MaterialInstanceDynamic))))
              (elif (== MaterialOverwrite 2)
                (goto _label_2)))))))))

(fn ConstructionScript)